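; Logo actor, in the Outro folder, that plays an animated UE4 logo and then quits the game.
; Construction creates a dynamic material instance on the logo plane.
; Animate restores normal time dilation, teleports the player's pawn to the actor, and drives the material's Phase through a timeline.
; It then plays an optional Matinee fade to black alongside a gamma-curved Fade timeline before quitting.
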(event `Animate`
  (bind _matinee_fade_to_black (`self.Matinee Fade to Black`))
  (`GameplayStatics.SetGlobalTimeDilation` 1.0)
  (`MaterialInstanceDynamic.SetScalarParameterValue` (`self.MID`) "Phase" 1.0)
  (`self.K2_TeleportTo` (`Controller.K2_GetPawn` (`GameplayStatics.GetPlayerController` 0)) (.location (`self.GetTransform`)) (.rotation (`self.GetTransform`)))
  (`KismetSystemLibrary.Delay` 0.5)
  (bind (_direction _phase) (`Timeline|Timeline_0` :!via `PlayFromStart`)
    (:`Update`
      (`MaterialInstanceDynamic.SetScalarParameterValue` (`self.MID`) "Phase" _phase))
    (:`Finished`
      (`KismetSystemLibrary.Delay` 0.5)
      (`/Engine/EditorBlueprintResources/StandardMacros.IsValid` _matinee_fade_to_black
        (:`Is Valid`
          (`MatineeActor.Play` _matinee_fade_to_black)
          (bind (_direction_2 _fade) (`Timeline|Timeline_1` :!via `PlayFromStart` :!label _label)
            (:`Update`
              (`MaterialInstanceDynamic.SetScalarParameterValue` (`self.MID`) "Fade" (`KismetMathLibrary.MultiplyMultiply_FloatFloat` _fade 2.2)))
            (:`Finished`
              (`KismetSystemLibrary.Delay` 0.75)
              (`KismetSystemLibrary.QuitGame` null "Quit"))))
        (:`Is Not Valid`
          (goto _label :!via `PlayFromStart`))))))

(event `self.ReceiveActorBeginOverlap`
  (params (OtherActor :type "Actor Object Reference")))

(event `self.ReceiveTick`
  (params (DeltaSeconds :type "Float (single-precision)")))

(fn `UserConstructionScript`
  (bind _returnvalue (`PrimitiveComponent.CreateDynamicMaterialInstance` (`self.UE4 Logo Plane`) 0 null))
  (bind _output_get (set `self.MID` _returnvalue))
  (`MaterialInstanceDynamic.SetScalarParameterValue` _output_get "Phase" 0.0))